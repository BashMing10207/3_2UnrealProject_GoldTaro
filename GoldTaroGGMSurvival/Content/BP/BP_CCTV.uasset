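; BP_CCTV is a possessable security camera that the player can view through and that sweeps side to side.
; Tick yaws the CineCamera at speed DIr, accumulating the angle travelled and reversing direction each time it passes 25 degrees.
; EnforceFunc calls PosCam to hand the player's controller to the camera.
; Tab repossesses Phone, the player pawn cached at BeginPlay.
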(event EventBeginPlay
  (Variables|Default|SetPhone (Game|Player|GetPlayerPawn 0)))

(event Collision|EventActorBeginOverlap
  (params (OtherActor :type Actor%20Object%20Reference)))

(event EventTick
  (params (DeltaSeconds :type Float%20%28single-precision%29))
  (Transformation|AddLocalRotation (Variables|Default|GetCineCamera) (Math|Rotator|MakeRotator 0.0 0.0 (* DeltaSeconds (Variables|Default|GetDIr))) false false)
  (bind _output_get (Variables|Default|Settemp (+ (Math|Float|Absolute(Float) (* DeltaSeconds (Variables|Default|GetDIr))) (Variables|Default|Gettemp))))
  (if (> _output_get 25.0)
    (Variables|Default|SetDIr (* (Variables|Default|GetDIr) -1.0))
    (Variables|Default|Settemp 0.0)))

(event EventPossessed
  (params (NewController :type Controller%20Object%20Reference)))

(event EventEnforceFunc
  (params (Owner :type Actor%20Object%20Reference))
  (CallFunction|PosCam (Pawn|GetController (Game|Player|GetPlayerPawn 0))))

(event Input|KeyboardEvents|Tab
  (params (Key :type Key%20Structure :default "None"))
  (:Pressed
    (Pawn|Possess (Pawn|GetController) (Variables|Default|GetPhone))))

(fn ConstructionScript)

(fn PosCam
  (params (NewParam :type Controller%20Object%20Reference))
  (Pawn|Possess NewParam self))