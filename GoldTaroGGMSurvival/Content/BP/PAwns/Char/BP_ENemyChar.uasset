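; Enemy character that wanders a linked node graph, starting just above its root node.
; After a random initial delay, TickV2V2 picks a random next node, or the root at dead ends, and sets a randomly timed timer, apparently to repeat itself.
; Tick reissues a move to the current target every frame through the AI controller, falling back to SimpleMoveToLocation.
; Node changes are time-driven, regardless of arrival.
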(event EventBeginPlay
  (bind _rootnode (Variables|Default|GetROotNode))
  (bind _output_get (Variables|Default|SetTarget (Transformation|GetActorLocation _rootnode)))
  (Transformation|SetActorLocation (+ _output_get "0.000000,0.000000,100.000000") false false)
  (Variables|Default|SetCurrentNode _rootnode)
  (Utilities|FlowControl|Delay (Math|Random|RandomFloatinRange (Variables|Default|GetDealyMin) (Variables|Default|GetDealyMax)))
  (CallFunction|TickV2V2))

(event Collision|EventActorBeginOverlap
  (params (OtherActor :type Actor%20Object%20Reference)))

(event EventTick
  (params (DeltaSeconds :type Float%20%28single-precision%29))
  (CallFunction|Tracing))

(fn ConstructionScript)

(fn TickV2V2
  (CallFunction|Move)
  (Utilities|Time|SetTimerbyEvent (EventDispatchers|CreateEvent :!event TickV2V2) (Math|Random|RandomFloatinRange (Variables|Default|GetDealyMin) (Variables|Default|GetDealyMax))))

(fn Tracing
  (bind _returnvalue (AI|GetAIController 0))
  (bind _target (Variables|Default|GetTarget))
  (if (Utilities|IsValid _returnvalue)
    (AI|Navigation|MovetoLocation _returnvalue _target -1.0 true true true true "/Script/NavigationSystem.RecastFilter_UseDefaultArea")
    (else
      (AI|Navigation|SimpleMovetoLocation (Pawn|GetController) _target))))

(fn Move
  (if (Utilities|Array|IsValidIndex (Variables|/Script/GoldTaroGGMSurvival.FN_EnemyMoveNode|GetNextNodes (Variables|Default|GetCurrentNode)))
    (Variables|Default|SetCurrentNode (.OutItem (Utilities|Array|Random (Variables|/Script/GoldTaroGGMSurvival.FN_EnemyMoveNode|GetNextNodes (Variables|Default|GetCurrentNode)))))
    (else
      (Variables|Default|SetCurrentNode (Variables|Default|GetROotNode))))
  (Variables|Default|SetTarget (Transformation|GetActorLocation (Variables|Default|GetCurrentNode))))