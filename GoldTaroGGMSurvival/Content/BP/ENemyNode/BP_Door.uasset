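; BP_Door is an electrically powered door actor that players toggle through Interact while it has power.
; OPenEvent slides the Door component between Open and Close marker positions, and applies the initial state on BeginPlay.
; Power events set IsPowered, with power loss forcing the door open.
; A self-rescheduling, random-interval InteracatOpen timer would drain slot energy while powered and closed, but nothing connected here starts it.
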(event Custom|OPenEvent
  (params (bIsOpen :type Boolean))
  (bind _output_get (Variables|Default|SetbIsOpended bIsOpen))
  (if _output_get
    (Components|MoveComponentTo (Variables|Default|GetDoor) (Variables|/Script/Engine.SceneComponent|GetRelativeLocation (Variables|Default|GetOpen)) "0, 0, 0" true false 0.2 false)
    (else
      (Components|MoveComponentTo (Variables|Default|GetDoor) (Variables|/Script/Engine.SceneComponent|GetRelativeLocation (Variables|Default|GetClose)) "0, 0, 0" true false 0.2 false))))

(event Custom|InteracatOpen
  (if (and (Variables|Default|GetIsPowered) (not (Variables|Default|GetbIsOpended)))
    (Class|IFNElectricContains|UseEnergy (Variables|Default|GetOwnerElectricSlot4) -1)
    (bind _returnvalue (Utilities|Time|SetTimerbyEvent (delegate Custom|InteracatOpen) (Math|Random|RandomFloatinRange 0.5 1e+01)))
    (Variables|Default|SetUseEnergyEventHandle _returnvalue)
    (elif (Utilities|Time|IsValidTimerHandle (Variables|Default|GetUseEnergyEventHandle))
      (Utilities|Time|PauseTimerbyHandle (Variables|Default|GetUseEnergyEventHandle)))))

(event EventBeginPlay
  (CallFunction|OPenEvent (Variables|Default|GetbIsOpended)))

(event Collision|EventActorBeginOverlap
  (params (OtherActor :type Actor%20Object%20Reference)))

(event EventTick
  (params (DeltaSeconds :type Float%20%28single-precision%29)))

(event EventTurnonEL
  (Variables|Default|SetIsPowered true))

(event EventTurnOffEl
  (Variables|Default|SetIsPowered false)
  (CallFunction|OPenEvent true))

(fn ConstructionScript)

(fn OpenClose
  (params (bIsOpen :type Boolean))
  (CallFunction|OPenEvent bIsOpen)
  (Development|PrintString "Hello"))

(fn Interact
  (params (playerArm :type FN%20Player%20Arm%20Object%20Reference) (caller :type Actor%20Object%20Reference))
  (if (Variables|Default|GetIsPowered)
    (CallFunction|OPenEvent (not (Variables|Default|GetbIsOpended)))
    (return 0)))