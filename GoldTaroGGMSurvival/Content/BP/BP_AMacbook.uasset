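; BP_AMacbook is an interactable, possessable laptop that works as a CCTV viewing terminal.
; Interact stores the calling player pawn in PlayerDir and has that pawn's controller possess the laptop.
; While possessed, key 1 cycles CamIndex through CCTVArray with wraparound, snapping the single Camera component to each CCTV actor's transform instead of switching view targets.
; Key 2 hands possession back to the stored player.
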(event EventBeginPlay)

(event Collision|EventActorBeginOverlap
  (params (OtherActor :type Actor%20Object%20Reference)))

(event EventTick
  (params (DeltaSeconds :type Float%20%28single-precision%29)))

(event EventInteract
  (params (player :type FN%20Player%20Character%20Object%20Reference))
  (bind _output_get (Variables|Default|SetPlayerDir player))
  (Pawn|Possess (Pawn|GetController _output_get) self))

(event Input|KeyboardEvents|1
  (params (Key :type Key%20Structure :default "None"))
  (bind _cctvarray (Variables|Default|GetCCTVArray))
  (:Pressed
    (bind _output_get (Variables|Default|SetCamIndex (Math|Integer|%(Integer) (+ (Variables|Default|GetCamIndex) 1) (Utilities|Array|Length _cctvarray))))
    (Transformation|SetWorldTransform (Variables|Default|GetCamera) (Transformation|GetActorTransform (Utilities|Array|Get(acopy) _cctvarray _output_get)) false false)))

(event Input|KeyboardEvents|2
  (params (Key :type Key%20Structure :default "None"))
  (:Pressed
    (Pawn|Possess (Pawn|GetController self) (Variables|Default|GetPlayerDir))))

(fn ConstructionScript)